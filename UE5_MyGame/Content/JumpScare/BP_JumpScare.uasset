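; BP_JumpScare is a jump scare actor that sends a mannequin toward an endpoint, then removes itself.
; While the CalledJumpscare flag is true, Tick moves the Mannequin in world space at constant Speed toward Endpoint, without sweeping.
; A Delay on the same Tick path destroys the actor three seconds after movement begins.
; Nothing in this Blueprint sets the trigger flag.
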(event EventTick
  (params (DeltaSeconds :type Float%20%28single-precision%29))
  (if (Variables|Default|GetCalledJumpscare)
    (Transformation|SetWorldLocation (Variables|Default|GetMannequin) (Math|Interpolation|VInterptoConstant (Transformation|GetWorldLocation (Variables|Default|GetMannequin)) (Transformation|GetWorldLocation (Variables|Default|GetEndpoint)) DeltaSeconds (Variables|Default|GetSpeed)) false false)
    (Utilities|FlowControl|Delay 3.0)
    (Actor|DestroyActor)))

(fn ConstructionScript)