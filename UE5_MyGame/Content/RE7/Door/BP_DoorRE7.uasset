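; Interactive RE7-style door that swings partly open, fully open or closed, away from or toward a side chosen by comparing player and door facing.
; HandleDoor picks a target yaw from the state Tick derives from current rotation, and a looping timer interpolates toward it until the player overlaps the box.
; Timer-driven checks auto-complete opening past a threshold and play open/close sounds; a velocity check handles creaking.
; Tick also prints debug state.
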(event OnComponentBeginOverlap(Box)
  (params (OverlappedComponent :type Primitive%20Component%20Object%20Reference) (OtherActor :type Actor%20Object%20Reference) (OtherComp :type Primitive%20Component%20Object%20Reference) (OtherBodyIndex :type Integer) (bFromSweep :type Boolean) (SweepResult :type Hit%20Result%20Structure%20%28by%20ref%29))
  (Utilities|Casting|CastToL1_Character OtherActor)
  (Utilities|Time|ClearandInvalidateTimerbyHandle (Variables|Default|GetTimer%20Reaming)))

(event Custom|StartInterectinDoor
  ;[0.15 0.15 0.15 0.5] TimerForRotating
  (bind _returnvalue (Utilities|Time|SetTimerbyEvent (delegate Custom|CustomEvent) 0.01 true))
  (Variables|Default|SetTimer%20Reaming _returnvalue))

(event Custom|CustomEvent
  ;[0.15 0.15 0.15 0.5] TimerForRotating
  (Transformation|SetRelativeRotation (Variables|Default|GetDoor) (Math|Rotator|MakeRotator 0.0 0.0 (Math|Interpolation|FInterptoConstant (.Yaw (Math|Rotator|BreakRotator (Variables|/Script/Engine.SceneComponent|GetRelativeRotation (Variables|Default|GetDoor)))) (Variables|Default|GetTargetAngle) (Utilities|Time|GetWorldDeltaSeconds) (Variables|Default|GetInterp%20Speed))) false false))

(event Custom|HandleDoor\
  ;[0.15 0.15 0.15 0.5] HandleDoor
  (switch Utilities|FlowControl|Switch|SwitchonE_DoorState (Variables|Default|GetDoorState)
    (:NewEnumerator0
      (bind _output_get (CallFunction|DoorSide))
      (bind _output_get_2 (Variables|Default|SetTargetAngle 15.0))
      (Variables|Default|SetTargetAngle (* _output_get_2 _output_get))
      (CallFunction|StartInterectinDoor))
    (:NewEnumerator1
      (bind _output_get_3 (CallFunction|DoorSide))
      (bind _output_get_4 (Variables|Default|SetTargetAngle 9e+01))
      (Variables|Default|SetTargetAngle (* _output_get_4 _output_get_3))
      (CallFunction|StartInterectinDoor))
    (:NewEnumerator2
      (CallFunction|DoorSide)
      (Variables|Default|SetTargetAngle 0.0)
      (CallFunction|StartInterectinDoor)
      (Physics|SetSimulatePhysics (Variables|Default|GetDoor) false))))

(event Custom|DoorSound
  (params (DoorState :type E_DoorState%20Enum :default "NewEnumerator0"))
  (bind _door (Variables|Default|GetDoor))
  (bind _returnvalue (Transformation|GetWorldLocation _door))
  (switch Utilities|FlowControl|Switch|SwitchonE_DoorState DoorState
    (:NewEnumerator0
      (Audio|PlaySoundatLocation "/Game/RE7/Door/Sound/Door_Close2.Door_Close2" _returnvalue "0, 0, 0" 1.0 1.0 0.0 0 0 0 0))
    (:NewEnumerator1
      (Audio|PlaySoundatLocation "/Game/RE7/Door/Sound/Door_Open.Door_Open" _returnvalue "0, 0, 0" 1.0 1.0 0.0 0 0 0 0))
    (:NewEnumerator2
      (Audio|PlaySoundatLocation "/Game/RE7/Door/Sound/Creaking-Door-Sound-Effect.Creaking-Door-Sound-Effect" _returnvalue "0, 0, 0" 1.0 1.0 0.0 0 0 0 0))))

(event Custom|Creaking
  ;[0.15 0.15 0.15 0.5] TimerForCreaking
  (if (== (.x (Transformation|GetComponentVelocity (Variables|Default|GetDoor))) 0.0)
    (Utilities|IsValid (Variables|Default|GetSoundCreaking)
      (:Is%20Valid
        (Audio|Components|Audio|Stop (Variables|Default|GetSoundCreaking)))
      (:Is%20Not%20Valid
        (goto _label Reset)))
    (else
      (Utilities|FlowControl|DoOnce true :!label _label
        (:Completed
          (bind _returnvalue (Audio|SpawnSoundAttached "/Game/RE7/Door/Sound/Creaking-Door-Sound-Effect.Creaking-Door-Sound-Effect" (Variables|Default|GetDoor) "None" "0, 0, 0" "0, 0, 0" "KeepRelativeOffset" false 1.0 1.0 (Math|Random|RandomFloatinRange 0.0 1e+01) 0 0))
          (Variables|Default|SetSoundCreaking _returnvalue))))))

(event Custom|SoundDoorOpenClose
  (bind _door (Variables|Default|GetDoor))
  (bind _relativerotation (Variables|/Script/Engine.SceneComponent|GetRelativeRotation _door))
  ;[0.15 0.15 0.15 0.5] TimerForSoundOpem
  (if (or (and (< (.yaw _relativerotation) 5.0) (> (.yaw _relativerotation) 0.0)) (and (> (.yaw _relativerotation) -5.0) (< (.yaw _relativerotation) -1.0)))
    (if (Variables|Default|GetOpened)
      (Utilities|IsValid (Variables|Default|GetSoundClose)
        (:Is%20Not%20Valid
          (bind _returnvalue (Audio|SpawnSoundAttached "/Game/RE7/Door/Sound/Door_Close2.Door_Close2" (Variables|Default|GetDoor) "None" "0, 0, 0" "0, 0, 0" "KeepRelativeOffset" false 1.0 1.0 0.0 0 0))
          (Variables|Default|SetSoundClose _returnvalue)
          (Utilities|FlowControl|RetriggerableDelay 0.2)
          (Variables|Default|SetOpened false)))
      (else
        (Utilities|IsValid (Variables|Default|GetSoundopen)
          (:Is%20Not%20Valid
            (bind _returnvalue_2 (Audio|SpawnSoundAttached "/Game/RE7/Door/Sound/Door_Open.Door_Open" (Variables|Default|GetDoor) "None" "0, 0, 0" "0, 0, 0" "KeepRelativeOffset" false 1.0 1.0 0.0 0 0))
            (Variables|Default|SetSoundopen _returnvalue_2)))))))

(event Custom|Closer
  (bind _door (Variables|Default|GetDoor))
  (bind _relativerotation (Variables|/Script/Engine.SceneComponent|GetRelativeRotation _door))
  ;[0.15 0.15 0.15 0.5] close sound
  (if (Utilities|Enum|Equal(Enum) (Variables|Default|GetDoorState) "NewEnumerator0")
    (goto _label Reset)
    (elif (or (and (> (.yaw _relativerotation) 66.0) (< (.yaw _relativerotation) 9e+01)) (and (< (.yaw _relativerotation) -66.0) (> (.yaw _relativerotation) -9e+01)))
      (Utilities|FlowControl|DoOnce false :!label _label
        (:Completed
          (CallFunction|AutoFullOpen))))))

(event Custom|AutoFullOpen
  ;[0.15 0.15 0.15 0.5] HandleDoor
  (bind _output_get (CallFunction|DoorSide))
  (bind _output_get_2 (Variables|Default|SetTargetAngle 9e+01))
  (Variables|Default|SetTargetAngle (* _output_get_2 _output_get))
  (CallFunction|StartInterectinDoor))

(event EventBeginPlay
  (bind _asl1_character (Utilities|Casting|CastToL1_Character (Game|GetPlayerCharacter 0)))
  ;[0.15 0.15 0.15 0.5] TimerForCreaking
  (Variables|Default|SetPlayer%20Ref _asl1_character)
  (Utilities|Time|SetTimerbyEvent (delegate Custom|Creaking) 0.0)
  (Utilities|Time|SetTimerbyEvent (delegate Custom|SoundDoorOpenClose) 0.01 true)
  ;[0.15 0.15 0.15 0.5] close sound
  (Utilities|Time|SetTimerbyEvent (delegate Custom|Closer) 0.01 true))

(event Collision|EventActorBeginOverlap
  (params (OtherActor :type Actor%20Object%20Reference)))

(event EventTick
  (params (DeltaSeconds :type Float%20%28single-precision%29))
  ;[0.15 0.15 0.15 0.5] Debugger
  (CallFunction|SetDoorState)
  (Development|PrintString (Utilities|String|EnumtoString (Variables|Default|GetDoorState)) true true "(R=0.000000,G=0.660000,B=1.000000,A=1.000000)" 0.01)
  (Development|PrintString (Utilities|String|ToString(Rotator) (Variables|/Script/Engine.SceneComponent|GetRelativeRotation (Variables|Default|GetDoor))) true true "(R=0.000000,G=0.660000,B=1.000000,A=1.000000)" 0.1)
  (Development|PrintString (Utilities|String|ToString(Boolean) (Variables|Default|GetOpened)) true true "(R=0.000000,G=0.660000,B=1.000000,A=1.000000)" 0.1))

(fn ConstructionScript)

(fn SetDoorState
  (bind _door (Variables|Default|GetDoor))
  (bind _relativerotation (Variables|/Script/Engine.SceneComponent|GetRelativeRotation _door))
  (if (or (and (>= (.yaw _relativerotation) 0.0) (< (.yaw _relativerotation) 1.0)) (and (<= (.yaw _relativerotation) 1.0) (> (.yaw _relativerotation) -1.0)))
    (Variables|Default|SetDoorState "NewEnumerator0")
    (if (Utilities|Enum|Equal(Enum) (Variables|Default|GetDoorState) "NewEnumerator0")
      (Variables|Default|SetInterp%20Speed 1e+01))
    (elif (or (and (> (.yaw _relativerotation) 1.0) (< (.yaw _relativerotation) 89.0)) (and (< (.yaw _relativerotation) -1.0) (> (.yaw _relativerotation) -89.0)))
      (Variables|Default|SetDoorState "NewEnumerator1")
      (Variables|Default|SetInterp%20Speed 9e+01)
      (elif (or (and (> (.yaw _relativerotation) 89.0) (< (.yaw _relativerotation) 91.0)) (and (< (.yaw _relativerotation) -89.0) (> (.yaw _relativerotation) -91.0)))
        (if (not (Utilities|Enum|Equal(Enum) (Variables|Default|GetDoorState) "NewEnumerator2"))
          (Variables|Default|SetDoorState "NewEnumerator2")
          (Variables|Default|SetInterp%20Speed 9e+01)
          (Variables|Default|SetOpened true)
          (Physics|SetSimulatePhysics (Variables|Default|GetDoor) false))))))

(fn DoorSide
  (if (< (Math|Vector|DotProduct (Math|Vector|GetForwardVector (Variables|/Game/GameBP/Level1/L1_Character.L1_Character_C|GetArrow1 (Variables|Default|GetPlayer%20Ref))) (Math|Vector|GetForwardVector (Variables|Default|GetArrow))) 0.0)
    (bind _output_get (Variables|Default|SetSideDoor -1.0))
    (return _output_get)
    (else
      (bind _output_get_2 (Variables|Default|SetSideDoor 1.0))
      (return _output_get_2))))