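; BP_Zombie is a zombie actor that takes damage and deals area melee damage to nearby pawns.
; AnyDamage subtracts damage from HP and destroys the zombie only when HP equals exactly zero, so overkill hits leave it alive.
; DealDamage runs a sphere overlap at AttackSphere using AttackRange, ignores itself, and applies BaseDamage to every pawn found.
; Each attack also draws a temporary red debug sphere showing the hit area.
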(event Custom|DealDamage
  (bind _attacksphere (Variables|Default|GetAttackSphere))
  (bind _returnvalue (Transformation|GetWorldLocation _attacksphere))
  (bind _outactors (Collision|SphereOverlapActors _returnvalue (Variables|Default|GetAttack%20Range) (Utilities|Array|MakeArray "ObjectTypeQuery3") "/Script/Engine.Actor" (Utilities|Array|MakeArray self)))
  (Rendering|Debug|DrawDebugSphere _returnvalue (Variables|Default|GetAttack%20Range) 12 "(R=1.000000,G=0.000000,B=0.000000,A=1.000000)" 2.0)
  (for _array_element _outactors
    (Game|Damage|ApplyDamage _array_element (Variables|Default|GetBase%20Damage) (Pawn|GetController) self "/Script/Engine.DamageType")))

(event Game|Damage|EventAnyDamage
  (params (Damage :type Float%20%28single-precision%29) (DamageType :type Damage%20Type%20Object%20Reference) (InstigatedBy :type Controller%20Object%20Reference) (DamageCauser :type Actor%20Object%20Reference))
  (Variables|Default|SetHP (- (Variables|Default|GetHP) Damage))
  (if (== (Variables|Default|GetHP) 0.0)
    (Actor|DestroyActor)))

(event EventBeginPlay)

(fn ConstructionScript)