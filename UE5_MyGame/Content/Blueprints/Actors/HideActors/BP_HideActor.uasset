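; Hiding spot actor that moves the player in or out on Interact, toggling the player's IsHiding state.
; A looping frame-delta timer slides the player at constant speed to HidingPosition or ExitPosition, then FinishedMoving fires a dispatcher.
; Entering disables collision, movement and inventory, and leaving restores them on arrival.
; The AIC_Classic enemy AI is asked whether it saw the player entering and is notified on exit; EnemyFound is empty.
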(event Custom|MoveCharacter
  (bind _player_ref (Variables|Default|GetPlayer%20Ref))
  ;[0.15 0.15 0.15 0.5] 여기까지 서랍장에 들어가는 것
  (Transformation|SetActorTransform _player_ref (Math|Transform|MakeTransform (Math|Interpolation|VInterptoConstant (Transformation|GetActorLocation _player_ref) (Transformation|GetWorldLocation (select (Variables|/Game/GameBP/Level1/L1_Character.L1_Character_C|GetIsHiding (Variables|Default|GetPlayer%20Ref)) (Variables|Default|GetExitPosition) (Variables|Default|GetHidingPosition))) (Utilities|Time|GetWorldDeltaSeconds) 1e+03) "0, 0, 0" "1.000000,1.000000,1.000000"))
  (if (Utilities|Operators|EqualEqual (Transformation|GetActorLocation (Variables|Default|GetPlayer%20Ref)) (Transformation|GetWorldLocation (select (Variables|/Game/GameBP/Level1/L1_Character.L1_Character_C|GetIsHiding (Variables|Default|GetPlayer%20Ref)) (Variables|Default|GetExitPosition) (Variables|Default|GetHidingPosition))) 0.01)
    (Utilities|Time|ClearandInvalidateTimerbyHandle (stale EventInteract _returnvalue_3))
    (Utilities|Time|ClearandInvalidateTimerbyHandle (stale EventInteract _returnvalue))
    (CallFunction|FinishedMoving)))

(event Custom|FinishedMoving
  (bind _player_ref (Variables|Default|GetPlayer%20Ref))
  (bind _player_ref_2 (Variables|Default|GetPlayer%20Ref))
  (Default|CallFinishedMoveingED)
  (if (Variables|/Game/GameBP/Level1/L1_Character.L1_Character_C|GetIsHiding _player_ref)
    (Variables|/Game/GameBP/Level1/L1_Character.L1_Character_C|SetIsHiding _player_ref false)
    (bind _asaic_classic (Utilities|Casting|CastToAIC_ClassicClass "/Game/AI/Classic/AIC_Classic.AIC_Classic_C"))
    (bind _returnvalue (Actor|GetActorOfClass _asaic_classic))
    (Class|BPIPlayerHiding|LeftHidingSpot(Message) _returnvalue)
    (Collision|SetActorEnableCollision _player_ref_2 true)
    (Pawn|Components|CharacterMovement|SetMovementMode (Variables|/Script/Engine.Character|GetCharacterMovement _player_ref_2) "MOVE_Walking" 0)
    (Variables|/Game/GameBP/HG_PlayerController.HG_PlayerController_C|SetCanOpenInventory (Variables|Default|GetControllerRef) true)
    (else
      (Variables|/Game/GameBP/Level1/L1_Character.L1_Character_C|SetIsHiding _player_ref true))))

(event Custom|EnemyFound)

(event EventBeginPlay
  (bind _asl1_character (Utilities|Casting|CastToL1_Character (Game|GetPlayerCharacter 0)))
  (Variables|Default|SetPlayer%20Ref _asl1_character)
  (bind _ashg_player_controller (Utilities|Casting|CastToHG_PlayerController (Game|GetPlayerController 0)))
  (Variables|Default|SetControllerRef _ashg_player_controller))

(event EventInteract
  (bind _player_ref (Variables|Default|GetPlayer%20Ref))
  (if (Variables|/Game/GameBP/Level1/L1_Character.L1_Character_C|GetIsHiding (Variables|Default|GetPlayer%20Ref))
    (bind _returnvalue (Utilities|Time|SetTimerbyEvent (delegate Custom|MoveCharacter) (Utilities|Time|GetWorldDeltaSeconds) true))
    (else
      (bind _asaic_classic (Utilities|Casting|CastToAIC_ClassicClass "/Game/AI/Classic/AIC_Classic.AIC_Classic_C"))
      (bind _returnvalue_2 (Actor|GetActorOfClass _asaic_classic))
      (Class|BPIPlayerHiding|DidEnemySee(Message) _returnvalue_2 self)
      (Collision|SetActorEnableCollision _player_ref false)
      (Pawn|Components|CharacterMovement|DisableMovement (Variables|/Script/Engine.Character|GetCharacterMovement _player_ref))
      (Variables|/Game/GameBP/HG_PlayerController.HG_PlayerController_C|SetCanOpenInventory (Variables|Default|GetControllerRef) false)
      (bind _returnvalue_3 (Utilities|Time|SetTimerbyEvent (delegate Custom|MoveCharacter) (Utilities|Time|GetWorldDeltaSeconds) true)))))

(fn ConstructionScript)