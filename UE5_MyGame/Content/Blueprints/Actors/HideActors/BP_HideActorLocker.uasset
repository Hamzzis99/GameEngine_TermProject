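; Locker hiding spot, a child hide actor that adds an animated swinging door.
; Interact locks further input, swings the door open with a timeline, then after a short delay hands off to the parent's interaction.
; The parent's finished-moving dispatcher triggers the door to close, which re-enables interaction.
; EnemyFound disables interaction and door collision, then swings the door open on a separate AI timeline.
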(event Custom|CloseDoor
  (bind _alpha (Timeline|CloseLockerDoor PlayFromStart)
    (:Update
      (Transformation|SetRelativeRotation (Variables|Default|GetStaticMesh1) (Math|Rotator|MakeRotator 0.0 0.0 (Math|Float|Lerp 9e+01 0.0 _alpha)) false false))
    (:Finished
      (Variables|Default|SetCanInteract true))))

(event Custom|FinishedMovingED_Event
  (Utilities|FlowControl|Delay 0.1)
  (CallFunction|CloseDoor))

(event EventBeginPlay
  (|CallParentFunction)
  (EventDispatchers|BindEventtoFinishedMoveingED (delegate Custom|FinishedMovingED_Event)))

(event EventEnemyFound
  (Variables|Default|SetCanInteract false)
  (Collision|SetCollisionEnabled (Variables|Default|GetStaticMesh1) "NoCollision")
  (bind _alpha (Timeline|AIOpenDoor PlayFromStart)
    (:Update
      (Transformation|SetRelativeRotation (Variables|Default|GetStaticMesh1) (Math|Rotator|MakeRotator 0.0 0.0 (Math|Float|Lerp 0.0 9e+01 _alpha)) false false))
    (:Finished
      (Utilities|FlowControl|Delay 0.2))))

(event EventInteract
  (if (Variables|Default|GetCanInteract)
    (Variables|Default|SetCanInteract false)
    (bind _alpha (Timeline|OpenLockerDoor PlayFromStart)
      (:Update
        (Transformation|SetRelativeRotation (Variables|Default|GetStaticMesh1) (Math|Rotator|MakeRotator 0.0 0.0 (Math|Float|Lerp 0.0 9e+01 _alpha)) false false))
      (:Finished
        (Utilities|FlowControl|Delay 0.2)
        (|CallParentFunction)))))

(fn ConstructionScript
  (|CallParentFunction))