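; Base pickup actor that lets the L1_Character collect an item into its inventory component.
; Overlapping the shape starts per-tick line traces to the player camera, showing a camera-facing prompt above the mesh when unobstructed.
; Trace distance toggles the prompt state and actor input, so the Action key works only within pickup range.
; Picking up adds the item, keeping any remainder on the actor or destroying it when none is left.
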(event OnComponentBeginOverlap(Shape)
  (params (OverlappedComponent :type Primitive%20Component%20Object%20Reference) (OtherActor :type Actor%20Object%20Reference) (OtherComp :type Primitive%20Component%20Object%20Reference) (OtherBodyIndex :type Integer) (bFromSweep :type Boolean) (SweepResult :type Hit%20Result%20Structure%20%28by%20ref%29))
  ;[0.15 0.15 0.15 0.5] Shape Collision 크기는 화살표를 가리키는 것.
  (bind _asl1_character (Utilities|Casting|CastToL1_Character OtherActor))
  (Variables|Default|SetPlayerRef _asl1_character)
  (Rendering|SetVisibility (Variables|Default|GetPromptWidget) true false)
  (Variables|Default|SetUpdateActor true))

(event OnComponentEndOverlap(Shape)
  (params (OverlappedComponent :type Primitive%20Component%20Object%20Reference) (OtherActor :type Actor%20Object%20Reference) (OtherComp :type Primitive%20Component%20Object%20Reference) (OtherBodyIndex :type Integer))
  ;[0.15 0.15 0.15 0.5] Shape Collision 크기는 화살표를 가리키는 것.
  (Utilities|Casting|CastToL1_Character OtherActor)
  (Rendering|SetVisibility (Variables|Default|GetPromptWidget) false false)
  (Variables|Default|SetUpdateActor false)
  (Input|DisableInput (Game|GetPlayerController 0)))

(event EventBeginPlay)

(event Collision|EventActorBeginOverlap
  (params (OtherActor :type Actor%20Object%20Reference)))

(event EventTick
  (params (DeltaSeconds :type Float%20%28single-precision%29))
  (bind _staticmesh (Variables|Default|GetStaticMesh))
  (bind _promptwidget (Variables|Default|GetPromptWidget))
  (bind _returnvalue (Transformation|GetWorldLocation _staticmesh))
  ;[0.15 0.15 0.15 0.5] 플레이어의 거리에 따라 이미지 회전 그리고. E키로 변경해주는...
  (Transformation|SetWorldLocation (Variables|Default|GetPromptWidget) (Math|Vector|MakeVector (.x _returnvalue) (.y _returnvalue) (+ (.z _returnvalue) (Variables|Default|GetWidgetDistanceAboveMesh))) false false)
  (if (Variables|Default|GetUpdateActor)
    ;;[0.15 0.15 0.15 0.5] 사물디버그 키고싶으면 Persistent 켜기.
    (bind (_outhit _returnvalue_2) (Collision|LineTraceByChannel (Transformation|GetActorLocation) (Transformation|GetWorldLocation (Variables|/Game/GameBP/Level1/L1_Character.L1_Character_C|GetCamera (Variables|Default|GetPlayerRef))) "TraceTypeQuery1" false 0 "None"))
    (if (not _returnvalue_2)
      (Rendering|SetVisibility _promptwidget true false)
      (Transformation|SetWorldRotation (Variables|Default|GetPromptWidget) (Math|Rotator|FindLookatRotation (Transformation|GetWorldLocation (Variables|Default|GetPromptWidget)) (Transformation|GetWorldLocation (Variables|/Game/GameBP/Level1/L1_Character.L1_Character_C|GetCamera (Variables|Default|GetPlayerRef)))) false false)
      (Default|TogglePrompt (.AsW%20Pickup%20Prompt (Utilities|Casting|CastToW_PickupPrompt (UserInterface|GetUserWidgetObject (Variables|Default|GetPromptWidget)))) (<= (Math|Vector|VectorLength (- (.TraceStart (Collision|BreakHitResult _outhit)) (.TraceEnd (Collision|BreakHitResult _outhit)))) (Variables|Default|GetPickUpDistance)))
      (if (<= (Math|Vector|VectorLength (- (.TraceStart (Collision|BreakHitResult _outhit)) (.TraceEnd (Collision|BreakHitResult _outhit)))) (Variables|Default|GetPickUpDistance))
        (Input|EnableInput (Game|GetPlayerController 0))
        (else
          (Input|DisableInput 0)))
      (else
        (Rendering|SetVisibility _promptwidget false false)
        (Input|DisableInput (Game|GetPlayerController 0))))))

(event Input|ActionEvents|InputActionAction
  (params (Key :type Key%20Structure :default "None"))
  ;[0.15 0.15 0.15 0.5] 아이템 줍기
  (:Pressed
    (CallFunction|PickUpItem)))

(fn ConstructionScript
  (Transformation|SetRelativeLocation (Variables|Default|GetPromptWidget) (Math|Vector|MakeVector 0.0 0.0 (Variables|Default|GetWidgetDistanceAboveMesh)) false false))

(fn PickUpItem
  (bind (_success_ _remainder) (Default|AddItem (Variables|/Game/GameBP/Level1/L1_Character.L1_Character_C|GetBPC_Inventory (Variables|Default|GetPlayerRef)) (Variables|Default|GetItem) (Variables|Default|GetAmount)))
  (if _success_
    (if (> _remainder 0)
      (Variables|Default|SetAmount _remainder)
      (return true)
      (else
        (Actor|DestroyActor)
        (return true)))
    (else
      (return false))))