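; Ammo box inventory item that gives the player extra ammunition when used.
; Its UseItem event adds a fixed amount to CharacterAmmo on PlayerRef, then sets UseItemSuccess to true, with no check on the current ammo count.
; The other events are disabled stubs, and the construction script only calls the parent.
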(event EventBeginPlay
  (|CallParentFunction) ; This node is disabled and will not be called.\nDrag off pins to build functionality.
)

(event Collision|EventActorBeginOverlap
  (params (OtherActor :type Actor%20Object%20Reference))
  (|CallParentFunction OtherActor) ; This node is disabled and will not be called.\nDrag off pins to build functionality.
)

(event EventTick
  (params (DeltaSeconds :type Float%20%28single-precision%29))
  (|CallParentFunction DeltaSeconds) ; This node is disabled and will not be called.\nDrag off pins to build functionality.
)

(event EventUseItem
  (bind _playerref (Variables|Default|GetPlayerRef))
  (Variables|/Game/GameBP/Level1/L1_Character.L1_Character_C|SetCharacter_Ammo _playerref (+ (Variables|/Game/GameBP/Level1/L1_Character.L1_Character_C|GetCharacter_Ammo _playerref) 15))
  (Variables|Default|SetUseItemSuccess true))

(fn ConstructionScript
  (|CallParentFunction))