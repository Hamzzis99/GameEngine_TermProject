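; BP_Inventory_Gun is an inventory item that arms the player with a pistol when used.
; UseItem sets HasWeapon on PlayerRef and shows the first-person mesh and weapon.
; It then starts the pistol reload montage on that mesh and immediately prints a Korean confirmation and flags UseItemSuccess, without waiting for the montage to finish.
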(event EventBeginPlay
  (|CallParentFunction) ; This node is disabled and will not be called.\nDrag off pins to build functionality.
)

(event Collision|EventActorBeginOverlap
  (params (OtherActor :type Actor%20Object%20Reference))
  (|CallParentFunction OtherActor) ; This node is disabled and will not be called.\nDrag off pins to build functionality.
)

(event EventTick
  (params (DeltaSeconds :type Float%20%28single-precision%29))
  (|CallParentFunction DeltaSeconds) ; This node is disabled and will not be called.\nDrag off pins to build functionality.
)

(event EventUseItem
  (bind _playerref (Variables|Default|GetPlayerRef))
  (bind _firstpersonmesh (Variables|/Game/GameBP/Level1/L1_Character.L1_Character_C|GetFirstPersonMesh _playerref))
  (Variables|/Game/GameBP/Level1/L1_Character.L1_Character_C|SetHasWeapon? _playerref true)
  (Rendering|SetVisibility _firstpersonmesh true false)
  (Rendering|SetVisibility (Variables|/Game/GameBP/Level1/L1_Character.L1_Character_C|GetWeapon _playerref) true false)
  (Animation|Montage|PlayMontage _firstpersonmesh "/Game/GameBP/Level1/GunHand/M1911/Animation/FP_PS_Reload_Montage.FP_PS_Reload_Montage"
    (:then
      (Development|PrintString "권총을 사용했습니다!")
      (Variables|Default|SetUseItemSuccess true))))

(fn ConstructionScript
  (|CallParentFunction))