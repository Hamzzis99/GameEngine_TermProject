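; RE8-style interactive door actor: interacting cracks it 15 degrees away from Closed, swings a partly open door to 90, or closes a fully open one.
; Tick derives the state from yaw and debug-prints it; a dot product between player and arrow picks swing direction.
; A looping timer interpolates yaw until the player overlaps the box.
; Other timers poll yaw and velocity for open, close and creak sounds.
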(event OnComponentBeginOverlap(Box)
  (params (OverlappedComponent :type Primitive%20Component%20Object%20Reference) (OtherActor :type Actor%20Object%20Reference) (OtherComp :type Primitive%20Component%20Object%20Reference) (OtherBodyIndex :type Integer) (bFromSweep :type Boolean) (SweepResult :type Hit%20Result%20Structure%20%28by%20ref%29))
  (Utilities|Casting|CastToL1_Character OtherActor)
  (Utilities|Time|ClearandInvalidateTimerbyHandle (Variables|Default|GetTimerRotating)))

(event Custom|HandleDoor
  (switch Utilities|FlowControl|Switch|SwitchonF_DoorState (Variables|Default|GetDoorState)
    (:NewEnumerator0
      (bind _output_get (CallFunction|DoorSide))
      (bind _output_get_2 (Variables|Default|SetTargetAngle 15.0))
      (Variables|Default|SetTargetAngle (* _output_get_2 _output_get))
      (CallFunction|StartInteractionDoor))
    (:NewEnumerator1
      (bind _output_get_3 (CallFunction|DoorSide))
      (bind _output_get_4 (Variables|Default|SetTargetAngle 9e+01))
      (Variables|Default|SetTargetAngle (* _output_get_4 _output_get_3))
      (CallFunction|StartInteractionDoor))
    (:NewEnumerator2
      (CallFunction|DoorSide)
      (Variables|Default|SetTargetAngle 0.0)
      (CallFunction|StartInteractionDoor))))

(event Custom|DoorSound
  (params (Door%20State :type F_DoorState%20Enum :default "NewEnumerator0"))
  (bind _door (Variables|Default|GetDoor))
  (bind _returnvalue (Transformation|GetWorldLocation _door))
  (switch Utilities|FlowControl|Switch|SwitchonF_DoorState Door%20State
    (:NewEnumerator0
      (Audio|PlaySoundatLocation "/Game/Sounds/RE7_Door/Door_Close2.Door_Close2" _returnvalue "0, 0, 0" 1.0 1.0 0.0 0 0 0 0))
    (:NewEnumerator1
      (Audio|PlaySoundatLocation "/Game/Sounds/RE7_Door/Door_Open.Door_Open" _returnvalue "0, 0, 0" 1.0 1.0 0.0 0 0 0 0))
    (:NewEnumerator2
      (Audio|PlaySoundatLocation "/Game/Sounds/RE7_Door/Creaking-Door-Sound-Effect.Creaking-Door-Sound-Effect" _returnvalue "0, 0, 0" 1.0 1.0 0.0 0 0 0 0))))

(event Custom|Creaking
  (if (== (.x (Transformation|GetComponentVelocity (Variables|Default|GetDoor))) 0.0)
    (Utilities|IsValid (Variables|Default|GetSound%20Creaking)
      (:Is%20Valid
        (Audio|Components|Audio|Stop (Variables|Default|GetSound%20Creaking)))
      (:Is%20Not%20Valid
        (goto _label Reset)))
    (else
      (Utilities|FlowControl|DoOnce true :!label _label
        (:Completed
          (bind _returnvalue (Audio|SpawnSoundAttached "/Game/Sounds/RE7_Door/Creaking-Door-Sound-Effect.Creaking-Door-Sound-Effect" (Variables|Default|GetDoor) "None" "0, 0, 0" "0, 0, 0" "KeepRelativeOffset" false 1.0 1.0 (Math|Random|RandomFloatinRange 0.0 1e+01) 0 0))
          (Variables|Default|SetSound%20Creaking _returnvalue))))))

(event Custom|SoundDooropenClose
  (bind _door (Variables|Default|GetDoor))
  (bind _relativerotation (Variables|/Script/Engine.SceneComponent|GetRelativeRotation _door))
  (if (or (and (< (.yaw _relativerotation) 5.0) (> (.yaw _relativerotation) 0.0)) (and (> (.yaw _relativerotation) -5.0) (< (.yaw _relativerotation) -1.0)))
    (if (Variables|Default|GetOpened)
      (Utilities|IsValid (Variables|Default|GetSound%20Close)
        (:Is%20Not%20Valid
          (bind _returnvalue (Audio|SpawnSoundAttached "/Game/Sounds/RE7_Door/Door_Close2.Door_Close2" (Variables|Default|GetDoor) "None" "0, 0, 0" "0, 0, 0" "KeepRelativeOffset" false 1.0 1.0 0.0 0 0))
          (Variables|Default|SetSound%20Close _returnvalue)
          (Utilities|FlowControl|RetriggerableDelay 0.2)
          (Variables|Default|SetOpened false)))
      (else
        ;[0.15 0.15 0.15 0.5] 시작 초반 문 열기 오픈 버그남
        (Utilities|IsValid (Variables|Default|GetSound%20Open)
          (:Is%20Not%20Valid
            (bind _returnvalue_2 (Audio|SpawnSoundAttached "/Game/Sounds/RE7_Door/Door_Open.Door_Open" (Variables|Default|GetDoor) "None" "0, 0, 0" "0, 0, 0" "KeepRelativeOffset" false 1.0 1.0 0.0 0 0))
            (Variables|Default|SetSound%20Open _returnvalue_2)))))))

(event Custom|Closer
  (bind _door (Variables|Default|GetDoor))
  (bind _relativerotation (Variables|/Script/Engine.SceneComponent|GetRelativeRotation _door))
  (if (Utilities|Enum|Equal(Enum) (Variables|Default|GetDoorState) "NewEnumerator0")
    (goto _label Reset)
    (elif (or (and (> (.yaw _relativerotation) 66.0) (< (.yaw _relativerotation) 9e+01)) (and (< (.yaw _relativerotation) -66.0) (> (.yaw _relativerotation) -9e+01)))
      (Utilities|FlowControl|DoOnce false :!label _label
        (:Completed
          (CallFunction|AutoFullopen))))))

(event Custom|AutoFullopen
  (bind _output_get (CallFunction|DoorSide))
  (bind _output_get_2 (Variables|Default|SetTargetAngle 9e+01))
  (Variables|Default|SetTargetAngle (* _output_get_2 _output_get))
  (CallFunction|StartInteractionDoor))

(event Custom|StartInteractionDoor
  (bind _returnvalue (Utilities|Time|SetTimerbyEvent (delegate Custom|CustomEvent) 0.01 true))
  (Variables|Default|SetTimerRotating _returnvalue))

(event Custom|CustomEvent
  (Transformation|SetRelativeRotation (Variables|Default|GetDoor) (Math|Rotator|MakeRotator 0.0 0.0 (Math|Interpolation|FInterptoConstant (.Yaw (Math|Rotator|BreakRotator (Variables|/Script/Engine.SceneComponent|GetRelativeRotation (Variables|Default|GetDoor)))) (Variables|Default|GetTargetAngle) (Utilities|Time|GetWorldDeltaSeconds) (Variables|Default|GetInterp%20Speed))) false false))

(event EventBeginPlay
  (bind _asl1_character (Utilities|Casting|CastToL1_Character (Game|GetPlayerCharacter 0)))
  (Variables|Default|SetPlayerRef _asl1_character)
  (Utilities|Time|SetTimerbyEvent (delegate Custom|Creaking) 0.01 true)
  (Utilities|Time|SetTimerbyEvent (delegate Custom|SoundDooropenClose) 0.01 true)
  (Utilities|Time|SetTimerbyEvent (delegate Custom|Closer) 0.0))

(event EventTick
  (params (DeltaSeconds :type Float%20%28single-precision%29))
  (CallFunction|SetDoorState)
  (Development|PrintString (Utilities|String|EnumtoString (Variables|Default|GetDoorState)) true true "(R=0.000000,G=0.660000,B=1.000000,A=1.000000)" 0.01)
  (Development|PrintString (Utilities|String|ToString(Rotator) (Variables|/Script/Engine.SceneComponent|GetRelativeRotation (Variables|Default|GetDoor))) true true "(R=0.000000,G=0.660000,B=1.000000,A=1.000000)" 0.01))

(fn ConstructionScript)

(fn SetDoorState
  (bind _door (Variables|Default|GetDoor))
  (bind _relativerotation (Variables|/Script/Engine.SceneComponent|GetRelativeRotation _door))
  (if (or (and (>= (.yaw _relativerotation) 0.0) (< (.yaw _relativerotation) 1.0)) (and (<= (.yaw _relativerotation) 0.0) (> (.yaw _relativerotation) -1.0)))
    (if (not (Utilities|Enum|Equal(Enum) (Variables|Default|GetDoorState) "NewEnumerator0"))
      (Variables|Default|SetDoorState "NewEnumerator0")
      (Variables|Default|SetInterp%20Speed 1e+01))
    (elif (or (and (>= (.yaw _relativerotation) 1.0) (< (.yaw _relativerotation) 89.0)) (and (< (.yaw _relativerotation) -1.0) (> (.yaw _relativerotation) -89.0)))
      (Variables|Default|SetDoorState "NewEnumerator1")
      (Variables|Default|SetInterp%20Speed 9e+01)
      (elif (or (and (>= (.yaw _relativerotation) 89.0) (< (.yaw _relativerotation) 91.0)) (and (< (.yaw _relativerotation) 89.0) (> (.yaw _relativerotation) -91.0)))
        (if (not (Utilities|Enum|Equal(Enum) (Variables|Default|GetDoorState) "NewEnumerator2"))
          (Variables|Default|SetDoorState "NewEnumerator2")
          (Variables|Default|SetInterp%20Speed 9e+01)
          (Variables|Default|SetOpened true)
          (Physics|SetSimulatePhysics (Variables|Default|GetDoor) false))))))

(fn DoorSide
  (if (< (Math|Vector|DotProduct (Math|Vector|GetForwardVector (Variables|/Game/GameBP/Level1/L1_Character.L1_Character_C|GetCharacter_NormalVector (Variables|Default|GetPlayerRef))) (Math|Vector|GetForwardVector (Variables|Default|GetArrow))) 0.0)
    (bind _output_get (Variables|Default|SetSideDoor -1.0))
    (return _output_get)
    (else
      (bind _output_get_2 (Variables|Default|SetSideDoor 1.0))
      (return _output_get_2))))